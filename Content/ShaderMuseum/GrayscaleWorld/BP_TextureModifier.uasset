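; Shader museum actor that renders an editable cloud noise material into a render target.
; BeginPlay creates a dynamic instance of MI_CloudNoiseDynamic on the Cube, and that instance is drawn to the render target immediately and again every Tick.
; DisplayWidgetForTexture lazily creates a WBP_MaterialEditorBasic widget bound to the same instance, or makes the existing one visible.
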(event EventBeginPlay
  (bind _returnvalue (Rendering|Material|CreateDynamicMaterialInstance (Variables|Default|GetCube) 0 "/Game/ShaderMuseum/GrayscaleWorld/MI_CloudNoiseDynamic.MI_CloudNoiseDynamic" "None" :!class /Script/Engine.PrimitiveComponent))
  (bind _output_get (Variables|Default|SetMaterial%20instance _returnvalue))
  (Rendering|DrawMaterialtoRenderTarget (Variables|Default|GetRenderTarget) _output_get))

(event EventTick
  (params (DeltaSeconds :type Float%20%28single-precision%29))
  (Rendering|DrawMaterialtoRenderTarget (Variables|Default|GetRenderTarget) (stale EventBeginPlay _output_get)))

(fn ConstructionScript
  (|CallParentFunction))

(fn DisplayWidgetforTexture
  (Utilities|IsValid (Variables|Default|GetWidget)
    (:Is%20Valid
      (Widget|SetVisibility (Variables|Default|GetWidget) "Visible"))
    (:Is%20Not%20Valid
      (bind _returnvalue (UserInterface|CreateWidget "/Game/ShaderMuseum/GrayscaleWorld/WBP_MaterialEditorBasic.WBP_MaterialEditorBasic_C" 0 (Variables|Default|GetMaterial%20instance)))
      (bind _output_get (Variables|Default|SetWidget _returnvalue))
      (UserInterface|Viewport|AddtoViewport _output_get 0))))